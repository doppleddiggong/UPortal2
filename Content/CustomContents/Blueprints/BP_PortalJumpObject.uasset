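; BP_PortalJumpObject is an object that can pass between an entry and exit portal door, using a duplicate mesh to show it at the exit.
; Activation reveals the copy and attaches it to the exit door.
; Each tick mirrors the original's entry-relative transform onto the copy, rotating only the location 180 degrees around the entry door's up vector.
; Deactivation hides the copy and moves the original to its world transform, completing the jump.
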(event EventActivateDuplicate
  (params (EntryDoor :type Scene%20Component%20Object%20Reference) (ExitDoor :type Scene%20Component%20Object%20Reference))
  (Variables|Default|SetEntry%20Door EntryDoor)
  (Variables|Default|SetExit%20Door ExitDoor)
  (Transformation|DetachFromComponent (Variables|Default|GetSM_Object_Copy) "KeepWorld" "KeepWorld" "KeepWorld" true)
  (Variables|Default|SetDuplicateActivate true)
  (Development|SetHiddeninGame (Variables|Default|GetSM_Object_Copy) false false)
  (Transformation|AttachComponentToComponent (Variables|Default|GetSM_Object_Copy) (Variables|Default|GetExit%20Door) "None" "KeepWorld" "KeepWorld" "KeepWorld" true))

(event EventTick
  (params (DeltaSeconds :type Float%20%28single-precision%29))
  (bind _entry_door (Variables|Default|GetEntry%20Door))
  (bind _sm_object (Variables|Default|GetSM_Object))
  (bind _returnvalue (Transformation|GetWorldTransform _sm_object))
  (bind _returnvalue_2 (Transformation|GetWorldTransform _entry_door))
  (bind _returnvalue_3 (Math|Transform|MakeRelativeTransform _returnvalue _returnvalue_2))
  (if (Variables|Default|GetDuplicateActivate)
    (Transformation|SetRelativeTransform (Variables|Default|GetSM_Object_Copy) (Math|Transform|MakeTransform (Math|Vector|RotateVectorAroundAxis (.location _returnvalue_3) 1.8e+02 (Math|Vector|GetUpVector _entry_door)) (.rotation _returnvalue_3) (.scale _returnvalue_3)) false false)))

(event EventDeactivateDuplicate
  (bind _sm_object_copy (Variables|Default|GetSM_Object_Copy))
  (if (Variables|Default|GetDuplicateActivate)
    (Variables|Default|SetDuplicateActivate false)
    (Development|SetHiddeninGame _sm_object_copy true false)
    (Transformation|SetWorldTransform (Variables|Default|GetSM_Object) (Transformation|GetWorldTransform _sm_object_copy) false false)))

(fn ConstructionScript)